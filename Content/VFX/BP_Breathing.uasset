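; BP_Breathing drives a breathing visual effect through Material Parameter Collections.
; Each Tick derives a target FOV that narrows as TargetBreathingValue rises, then eases FOV and BreathingValue toward their targets with FInterpTo.
; The smoothed values are written to MPC_Focus for FOV and MPC_Breathing for post-process.
; An IsBreathing branch that would set both targets is disconnected, so this graph never changes TargetBreathingValue.
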(event EventTick
  (params (DeltaSeconds :type Float%20%28single-precision%29))
  (Utilities|FlowControl|Sequence
    (:then_0
      ;[0.15 0.15 0.15 0.5] Breathing Effect
      ;;[0.15 0.15 0.15 0.5] set fov
      (bind _output_get (Variables|Default|SetTargetFOV (- 1.0 (* (Variables|Default|GetTargetBreathingValue) 0.2)))))
    (:then_1
      (Utilities|FlowControl|Sequence
        (:then_0
          ;;[0.15 0.15 0.15 0.5] FOV
          (bind _output_get_2 (Variables|Default|SetFOV (Math|Interpolation|FInterpTo (Variables|Default|GetFOV) (Variables|Default|GetTargetFOV) DeltaSeconds 2.0)))
          (Rendering|Material|SetScalarParameterValue "/Game/VFX/MPC_Focus.MPC_Focus" "FOV" _output_get_2 :!class /Script/Engine.KismetMaterialLibrary))
        (:then_1
          ;;[0.15 0.15 0.15 0.5] Post-Process
          (bind _output_get_3 (Variables|Default|SetBreathingValue (Math|Interpolation|FInterpTo (Variables|Default|GetBreathingValue) (Variables|Default|GetTargetBreathingValue) DeltaSeconds 2.0)))
          (Rendering|Material|SetScalarParameterValue "/Game/VFX/MPC_Breathing.MPC_Breathing" "BreathingValue" _output_get_3 :!class /Script/Engine.KismetMaterialLibrary))))))