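; Rocket launch desk where the player adjusts two handles and confirms to launch the rocket.
; Clicking Left or Right selects that handle; Tick then turns controller scroll input into bounded value changes and vertical marker movement.
; Confirm only requires both handles to have been clicked, then a timeline switches to top-down view, restores movement and calls Lunchhh on every update.
; The proximity box sets CanAdjust, which nothing here reads.
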(event OnComponentBeginOverlap(Box)
  (params (OverlappedComponent :type Primitive%20Component%20Object%20Reference) (OtherActor :type Actor%20Object%20Reference) (OtherComp :type Primitive%20Component%20Object%20Reference) (OtherBodyIndex :type Integer) (bFromSweep :type Boolean) (SweepResult :type Hit%20Result%20Structure%20%28by%20ref%29))
  ;[0.15 0.15 0.15 0.5] 进出盒子开关提示
  (Utilities|Casting|CastToBP_TopDownCharacter OtherActor)
  (Variables|Default|SetCanAdjust true))

(event OnClicked(Right)
  (params (TouchedComponent :type Primitive%20Component%20Object%20Reference) (ButtonPressed :type Key%20Structure :default "None"))
  ;[0.15 0.15 0.15 0.5] 选择零件按钮
  (Variables|Default|SetIfRightAdjust true)
  (Variables|Default|SetRightHandleSelected true)
  (Variables|Default|SetLeftHandleSelected false))

(event OnComponentEndOverlap(Box)
  (params (OverlappedComponent :type Primitive%20Component%20Object%20Reference) (OtherActor :type Actor%20Object%20Reference) (OtherComp :type Primitive%20Component%20Object%20Reference) (OtherBodyIndex :type Integer))
  ;[0.15 0.15 0.15 0.5] 进出盒子开关提示
  (Utilities|Casting|CastToBP_TopDownCharacter OtherActor)
  (Variables|Default|SetCanAdjust false))

(event OnClicked(Left)
  (params (TouchedComponent :type Primitive%20Component%20Object%20Reference) (ButtonPressed :type Key%20Structure :default "None"))
  ;[0.15 0.15 0.15 0.5] 选择零件按钮
  (Variables|Default|SetIfLeftAdjust true)
  (Variables|Default|SetLeftHandleSelected true)
  (Variables|Default|SetRightHandleSelected false))

(event OnClicked(Comfirm)
  (params (TouchedComponent :type Primitive%20Component%20Object%20Reference) (ButtonPressed :type Key%20Structure :default "None"))
  ;[0.15 0.15 0.15 0.5] 火箭完成按钮
  (if (and (Variables|Default|GetIfRightAdjust) (Variables|Default|GetIfLeftAdjust))
    (Development|PrintString "火箭f发射！")
    ;[0.15 0.15 0.15 0.5] 改变视角到topdown
    (bind _camerazoomin (Timeline|Timeline PlayFromStart)
      (:Update
        (Default|ChangeViewtoTopDown (Variables|Default|GetRoketDesk) _camerazoomin)
        (Variables|/Game/LunchMeow/Blueprints/RoketDesk.RoketDesk_C|SetStartBuilding (Variables|Default|GetRoketDesk) false)
        (Variables|/Game/TopDown/Blueprints/BP_TopDownController.BP_TopDownController_C|SetIsMovable (Variables|Default|GetPlayerController) true)
        (Variables|Default|SetFinishAdjust true)
        (Default|Lunchhh (Variables|Default|GetWholeRokect))))
    (else
      (Development|PrintString "火箭参数未调整完"))))

(event EventBeginPlay
  ;[0.15 0.15 0.15 0.5] 获得玩家手里的滚轮数据
  (Utilities|FlowControl|Sequence
    (:then_0
      (bind _returnvalue (Actor|GetActorOfClass "/Game/TopDown/Blueprints/BP_TopDownController.BP_TopDownController_C"))
      (Variables|Default|SetBP_Player _returnvalue)
      (bind _returnvalue_2 (Actor|GetActorOfClass "/Game/LunchMeow/Blueprints/RoketDesk.RoketDesk_C"))
      (Variables|Default|SetRoketDesk _returnvalue_2)
      (bind _returnvalue_3 (Actor|GetActorOfClass "/Game/TopDown/Blueprints/BP_TopDownController.BP_TopDownController_C"))
      (Variables|Default|SetPlayerController _returnvalue_3)
      (bind _returnvalue_4 (Actor|GetActorOfClass "/Game/LunchMeow/Blueprints/WholeRoket.WholeRoket_C"))
      (Variables|Default|SetWholeRokect _returnvalue_4)
      (bind _returnvalue_5 (Actor|GetActorOfClass "/Game/LunchMeow/Blueprints/UISystem.UISystem_C"))
      (Variables|Default|SetUISystem _returnvalue_5))))

(event EventTick
  (params (DeltaSeconds :type Float%20%28single-precision%29))
  (Utilities|FlowControl|Sequence
    (:then_0
      ;[0.15 0.15 0.15 0.5] 右手拉杆子
      (if (Variables|Default|GetRightHandleSelected)
        (Utilities|FlowControl|Sequence
          (:then_0
            (Utilities|RightHandleValueChange (Variables|Default|GetRightRecord) 1 true 0.05 20))
          (:then_1
            (Utilities|RightHandleValueChange (Variables|Default|GetRightRecord) -1 false 0.05 20)))))
    (:then_1
      ;[0.15 0.15 0.15 0.5] 左手拉杆子
      (if (Variables|Default|GetLeftHandleSelected)
        (Utilities|FlowControl|Sequence
          (:then_0
            (Utilities|LeftHandleValueChange (Variables|Default|GetLeftRocrd) 1 true 0.05 20))
          (:then_1
            (Utilities|LeftHandleValueChange (Variables|Default|GetLeftRocrd) -1 false 0.05 20)))))))

(fn ConstructionScript)