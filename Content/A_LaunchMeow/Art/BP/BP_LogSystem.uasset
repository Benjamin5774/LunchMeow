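; BP_LogSystem is an actor that feeds note text into a black box log UI.
; BeginPlay gathers lines from Notes into an array, caches the Dialogue widget and looks up the game manager, controller and character.
; Every Tick, RunNotesByIndex loops to the CurrentIndex entry and writes its Components, Astronaut and Variables texts to the player character's WBPLog, not the cached one.
; CurrentIndex is not changed within this Blueprint.
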(event EventBeginPlay
  (bind _notes (Variables|Default|GetNotes))
  (bind (_line0 _line1 _line2 _line3 _line4 _line5 _line6 _line7 _line8 _line9 _line10 _line11 _line12 _line13) (Utilities|Struct|BreakStructure_Notes _notes))
  (Utilities|FlowControl|Sequence
    (:then_0
      ;[0.15 0.15 0.15 0.5] 初始化Alice对话
      (Variables|Default|SetEachNotes (Utilities|Array|MakeArray _line0 _line1 _line2 _line3 _line4 _line5 _line6 _line7 _line8 _line9 _line10 _line11 _line12 _line13 "")))
    (:then_1
      ;[0.15 0.15 0.15 0.5] 获取日志UI
      (bind _aseuw_black_box_log (Utilities|Casting|CastToEUW_BlackBoxLog (UserInterface|GetWidget (Variables|Default|GetDialogue))))
      (Variables|Default|SetWBPLog _aseuw_black_box_log))
    (:then_2
      ;[0.15 0.15 0.15 0.5] 获取GM
      (bind _returnvalue (Actor|GetActorOfClass "/Game/LunchMeow/Blueprints/GameManager.GameManager_C"))
      (Variables|Default|SetGameManager _returnvalue))
    (:then_3
      ;[0.15 0.15 0.15 0.5] 获得PlayerControl
      (bind _returnvalue_2 (Actor|GetActorOfClass "/Game/TopDown/Blueprints/BP_TopDownController.BP_TopDownController_C"))
      (Variables|Default|SetPlayerControl _returnvalue_2)
      (bind _returnvalue_3 (Actor|GetActorOfClass "/Game/TopDown/Blueprints/BP_TopDownCharacter.BP_TopDownCharacter_C"))
      (Variables|Default|SetPlayerCharacter _returnvalue_3))))

(event EventTick
  (params (DeltaSeconds :type Float%20%28single-precision%29))
  (CallFunction|RunNotesbyIndex (Variables|Default|GetEachNotes) (Variables|Default|GetCurrentIndex)))

(fn ConstructionScript)

(fn RunNotesbyIndex
  (params (EachLine :type Array%20of%20Structure%20Note%20Structures) (CurrentLine :type Integer))
  (bind _playercharacter (Variables|Default|GetPlayerCharacter))
  (bind _wbplog (Variables|/Game/TopDown/Blueprints/BP_TopDownCharacter.BP_TopDownCharacter_C|GetWBPLog _playercharacter))
  (bind (_array_element _array_index) (Utilities|Array|ForEachLoopwithBreak EachLine)
    (:LoopBody
      (if (== _array_index CurrentLine)
        (Rendering|Components|TextRender|SetText (Variables|/Game/211/04_EUW/EUW_BlackBoxLog.EUW_BlackBoxLog_C|GetComponents _wbplog) (Utilities|Text|ToText(String) (Utilities|String|ToString(Text) (.Components (Utilities|Struct|BreakStructure_Note _array_element)))))
        (Rendering|Components|TextRender|SetText (Variables|/Game/211/04_EUW/EUW_BlackBoxLog.EUW_BlackBoxLog_C|GetAstronaut _wbplog) (Utilities|Text|ToText(String) (Utilities|String|ToString(Text) (.Astru (Utilities|Struct|BreakStructure_Note _array_element)))))
        (Rendering|Components|TextRender|SetText (Variables|/Game/211/04_EUW/EUW_BlackBoxLog.EUW_BlackBoxLog_C|GetVariables _wbplog) (Utilities|Text|ToText(String) (Utilities|String|ToString(Text) (.Variables (Utilities|Struct|BreakStructure_Note _array_element)))))))))