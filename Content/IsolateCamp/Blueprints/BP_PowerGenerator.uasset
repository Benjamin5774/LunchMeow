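; BP_PowerGenerator is an animated power generator prop in the IsolateCamp content, with three ring components that spin continuously.
; Each Tick rotates Ring1, Ring2 and Ring3 around their local yaw axis, each at its own rate variable scaled by DeltaSeconds for frame-rate-independent motion.
; BeginPlay, overlap and the construction script contain no logic, so the motion is purely visual.
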(event EventBeginPlay)

(event Collision|EventActorBeginOverlap
  (params (OtherActor :type Actor%20Object%20Reference)))

(event EventTick
  (params (DeltaSeconds :type Float%20%28single-precision%29))
  (Transformation|AddLocalRotation (Variables|Default|GetRing3) (Math|Rotator|MakeRotator 0.0 0.0 (* (Variables|Default|GetRotation20) DeltaSeconds)) false false)
  (Transformation|AddLocalRotation (Variables|Default|GetRing2) (Math|Rotator|MakeRotator 0.0 0.0 (* (Variables|Default|GetRotation10) DeltaSeconds)) false false)
  (Transformation|AddLocalRotation (Variables|Default|GetRing1) (Math|Rotator|MakeRotator 0.0 0.0 (* (Variables|Default|GetRotation30) DeltaSeconds)) false false))

(fn ConstructionScript)