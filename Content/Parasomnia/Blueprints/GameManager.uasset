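; GameManager Blueprint that tracks the game state and right-focus flags for SIMA and SHALOU.
; StartGame, PauseGame and BackToMenu each set the current state enum and toggle pause, with only StartGame unpausing.
; Simple setter events switch the two focus booleans on and off independently.
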(event Custom|setSHALOUTrue
  (Variables|Default|SetisSHALOURightFocused true))

(event Custom|setSIMATrue
  (Variables|Default|SetisSIMARightFocused true))

(event Custom|setSIMAFlase
  (Variables|Default|SetisSIMARightFocused false))

(event Custom|setSHALOUFlase
  (Variables|Default|SetisSHALOURightFocused false))

(fn StartGame()
  (Variables|Default|SetCurrentGameState "NewEnumerator2")
  (Game|SetGamePaused false))

(fn PauseGame()
  (Variables|Default|SetCurrentGameState "NewEnumerator3")
  (Game|SetGamePaused true))

(fn BacktoMenu()
  (Variables|Default|SetCurrentGameState "NewEnumerator1")
  (Game|SetGamePaused true))