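; Dialogue actor that plays Alice's fifteen-line conversation on the player character's screen UI.
; BeginPlay builds the line array and caches its dialogue widget, GameManager, top-down controller and character.
; While GameManager.CanTalk and IsTalkToAlice are set, Tick writes the CurrentIndex line's speaker and text through RunDialogueByIndex.
; Once the index, which is advanced outside these graphs, exceeds the array length, it clears both flags and the controller's IsDialogueHide.
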(event EventBeginPlay
  (bind _alicedialogue (Variables|Default|GetAliceDialogue))
  (bind (_line0 _line1 _line2 _line3 _line4 _line5 _line6 _line7 _line8 _line9 _line10 _line11 _line12 _line13 _line14) (Utilities|Struct|BreakAlice _alicedialogue))
  (Utilities|FlowControl|Sequence
    (:then_0
      ;[0.15 0.15 0.15 0.5] 初始化Alice对话
      (Variables|Default|SetAliceEachLine (Utilities|Array|MakeArray _line0 _line1 _line2 _line3 _line4 _line5 _line6 _line7 _line8 _line9 _line10 _line11 _line12 _line13 _line14)))
    (:then_1
      ;[0.15 0.15 0.15 0.5] 获取对话UI
      (bind _aswbp_dialogue (Utilities|Casting|CastToWBP_Dialogue (UserInterface|GetWidget (Variables|Default|GetDialogue))))
      (Variables|Default|SetDialogueUI _aswbp_dialogue))
    (:then_2
      ;[0.15 0.15 0.15 0.5] 获取GM
      (bind _returnvalue (Actor|GetActorOfClass "/Game/LunchMeow/Blueprints/GameManager.GameManager_C"))
      (Variables|Default|SetGameManager _returnvalue))
    (:then_3
      ;[0.15 0.15 0.15 0.5] 获得PlayerControl
      (bind _returnvalue_2 (Actor|GetActorOfClass "/Game/TopDown/Blueprints/BP_TopDownController.BP_TopDownController_C"))
      (Variables|Default|SetPlayerControl _returnvalue_2)
      (bind _returnvalue_3 (Actor|GetActorOfClass "/Game/TopDown/Blueprints/BP_TopDownCharacter.BP_TopDownCharacter_C"))
      (Variables|Default|SetPlayerCharacter _returnvalue_3))))

(event EventTick
  (params (DeltaSeconds :type Float%20%28single-precision%29))
  (bind _currentindex (Variables|Default|GetCurrentIndex))
  (if (Variables|/Game/LunchMeow/Blueprints/GameManager.GameManager_C|GetCanTalk (Variables|Default|GetGameManager))
    (Utilities|FlowControl|Sequence
      (:then_0
        ;[0.15 0.15 0.15 0.5] 和下属Alice对话
        (if (Variables|Default|GetIsTalkToAlice)
          ;;[0.15 0.15 0.15 0.5] 数组index判定
          (if (<= (Variables|Default|GetCurrentIndex) (Utilities|Array|Length (Variables|Default|GetAliceEachLine)))
            (CallFunction|RunDialoguebyIndex (Variables|Default|GetAliceEachLine) _currentindex)
            (Development|PrintString (Utilities|String|ToString(Integer) _currentindex))
            (else
              (Variables|Default|SetIsTalkToAlice false)
              (Variables|/Game/LunchMeow/Blueprints/GameManager.GameManager_C|SetCanTalk (Variables|Default|GetGameManager) false)
              (Variables|/Game/TopDown/Blueprints/BP_TopDownController.BP_TopDownController_C|SetIsDialogueHide (Variables|Default|GetPlayerControl) false))))))))

(fn ConstructionScript)

(fn RunDialoguebyIndex
  (params (EachLine :type Array%20of%20ST%20Dialogue%20Structures) (CurrentLine :type Integer))
  (bind _playercharacter (Variables|Default|GetPlayerCharacter))
  (bind _dialoguescreenui_ (Variables|/Game/TopDown/Blueprints/BP_TopDownCharacter.BP_TopDownCharacter_C|GetDialogueScreenUI%20 _playercharacter))
  (bind (_array_element _array_index) (Utilities|Array|ForEachLoopwithBreak EachLine)
    (:LoopBody
      (if (== _array_index CurrentLine)
        (Rendering|Components|TextRender|SetText (Variables|/Game/LunchMeow/UI/WBP_Dialogue.WBP_Dialogue_C|GetText_Speaker _dialoguescreenui_) (Utilities|Text|ToText(String) (.Speaker (Utilities|Struct|BreakST_Dialogue _array_element))))
        (Rendering|Components|TextRender|SetText (Variables|/Game/LunchMeow/UI/WBP_Dialogue.WBP_Dialogue_C|GetText_Line _dialoguescreenui_) (.Text (Utilities|Struct|BreakST_Dialogue _array_element)))))))