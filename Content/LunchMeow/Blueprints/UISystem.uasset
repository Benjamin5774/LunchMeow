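; UISystem is an actor that shows guidance prompts on the player's screen as they move between the rocket desk, lunch desk and cat room tasks.
; BeginPlay caches the desks, character, GameManager and CatSystem and builds the guidance line array.
; Tick polls their flags and writes the matching line to the character's GuidanceScreenUI, skipping the fourth line.
; SetTextToNull's clearing code is disconnected, so prompts are never blanked here.
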(event EventBeginPlay
  (bind _guidances (Variables|Default|GetGuidances))
  (bind (_line0 _line1 _line2 _line3 _line4 _line5) (Utilities|Struct|BreakUIGuidance _guidances))
  (Utilities|FlowControl|Sequence
    (:then_0
      ;[0.15 0.15 0.15 0.5] 获得UI系统
      (bind _aswbp_ui (Utilities|Casting|CastToWBP_UI (UserInterface|GetWidget (Variables|Default|GetUI))))
      (Variables|Default|SetUISystem _aswbp_ui))
    (:then_1
      ;[0.15 0.15 0.15 0.5] 初始化引导UI
      (Variables|Default|SetGuidanceEachLine (Utilities|Array|MakeArray _line0 _line1 _line2 _line3 _line4 _line5)))
    (:then_2
      ;[0.15 0.15 0.15 0.5] 获取火箭桌面
      (bind _returnvalue (Actor|GetActorOfClass "/Game/LunchMeow/Blueprints/RoketDesk.RoketDesk_C"))
      (Variables|Default|SetRoketDesk _returnvalue)
      (bind _returnvalue_2 (Actor|GetActorOfClass "/Game/LunchMeow/Blueprints/LunchDesk.LunchDesk_C"))
      (Variables|Default|SetLunchDesk _returnvalue_2))
    (:then_3
      ;[0.15 0.15 0.15 0.5] 获取角色
      (bind _returnvalue_3 (Actor|GetActorOfClass "/Game/TopDown/Blueprints/BP_TopDownCharacter.BP_TopDownCharacter_C"))
      (Variables|Default|SetPlayerCharacter _returnvalue_3)
      (bind _returnvalue_4 (Actor|GetActorOfClass "/Game/LunchMeow/Blueprints/GameManager.GameManager_C"))
      (Variables|Default|SetGameManager _returnvalue_4)
      (bind _returnvalue_5 (Actor|GetActorOfClass "/Game/LunchMeow/Blueprints/CatSystem.CatSystem_C"))
      (Variables|Default|SetCatSystem _returnvalue_5))))

(event EventTick
  (params (DeltaSeconds :type Float%20%28single-precision%29))
  (bind _catsystem (Variables|Default|GetCatSystem))
  (bind _roketdesk (Variables|Default|GetRoketDesk))
  (bind _lunchdesk (Variables|Default|GetLunchDesk))
  (bind _canbuild (Variables|/Game/LunchMeow/Blueprints/RoketDesk.RoketDesk_C|GetCanBuild _roketdesk))
  (bind _canadjust (Variables|/Game/LunchMeow/Blueprints/LunchDesk.LunchDesk_C|GetCanAdjust _lunchdesk))
  (bind _returnvalue (or _canbuild _canadjust))
  (Utilities|FlowControl|Sequence
    (:then_0
      (if _returnvalue
        (if (Variables|/Game/LunchMeow/Blueprints/RoketDesk.RoketDesk_C|GetCanBuild (Variables|Default|GetRoketDesk))
          ;[0.15 0.15 0.15 0.5] 展示第一句引导
          (CallFunction|RunGuidancebyIndex (Variables|Default|GetGuidanceEachLine))
          (Variables|Default|SetHideUI false)
          (elif (Variables|/Game/LunchMeow/Blueprints/LunchDesk.LunchDesk_C|GetCanAdjust (Variables|Default|GetLunchDesk))
            ;[0.15 0.15 0.15 0.5] 展示第二句引导
            (CallFunction|RunGuidancebyIndex (Variables|Default|GetGuidanceEachLine) 1)
            (Variables|Default|SetHideUI false)))
        (else
          ;[0.15 0.15 0.15 0.5] 不靠近的时候显示空值
          (CallFunction|SetTexttoNull))))
    (:then_1
      ;[0.15 0.15 0.15 0.5] 展示第三句引导
      (if (Variables|/Game/LunchMeow/Blueprints/GameManager.GameManager_C|GetGuidanceToRocketDesk (Variables|Default|GetGameManager))
        (CallFunction|RunGuidancebyIndex (Variables|Default|GetGuidanceEachLine) 2)
        (elif (not _returnvalue)
          (Utilities|FlowControl|DoOnce false
            (:Completed
              (CallFunction|SetTexttoNull))))))
    (:then_2
      ;[0.15 0.15 0.15 0.5] 展示第五句引导
      (if (Variables|/Game/LunchMeow/Blueprints/GameManager.GameManager_C|GetGuidanceToCatRoom (Variables|Default|GetGameManager))
        (CallFunction|RunGuidancebyIndex (Variables|Default|GetGuidanceEachLine) 4)
        (elif (Variables|/Game/LunchMeow/Blueprints/RoketDesk.RoketDesk_C|GetFInishBuild (Variables|Default|GetRoketDesk))
          (Utilities|FlowControl|DoOnce false
            (:Completed
              (CallFunction|SetTexttoNull))))))
    (:then_3
      ;[0.15 0.15 0.15 0.5] 展示第六句引导
      (if (Variables|/Game/LunchMeow/Blueprints/GameManager.GameManager_C|GetGuidanceToLunchRoom (Variables|Default|GetGameManager))
        (CallFunction|RunGuidancebyIndex (Variables|Default|GetGuidanceEachLine) 5)
        (elif (and (Variables|/Game/LunchMeow/Blueprints/CatSystem.CatSystem_C|GetIsSeat1Finish _catsystem) (Variables|/Game/LunchMeow/Blueprints/CatSystem.CatSystem_C|GetIsSeat2Finish _catsystem))
          (Utilities|FlowControl|DoOnce false
            (:Completed
              (CallFunction|SetTexttoNull))))))))

(fn ConstructionScript)

(fn RunGuidancebyIndex
  (params (EachGuidance :type Array%20of%20ST%20UI%20Structures) (CurrentIndex :type Integer))
  (bind (_array_element _array_index) (Utilities|Array|ForEachLoopwithBreak EachGuidance)
    (:LoopBody
      (if (== _array_index CurrentIndex)
        (Rendering|Components|TextRender|SetText (Variables|/Game/LunchMeow/UI/WBP_UI.WBP_UI_C|GetUI_Guidance (Variables|/Game/TopDown/Blueprints/BP_TopDownCharacter.BP_TopDownCharacter_C|GetGuidanceScreenUI (Variables|Default|GetPlayerCharacter))) (Utilities|Text|ToText(String) (Utilities|String|ToString(Text) (.Text (Utilities|Struct|BreakST_UI _array_element)))))))))

(fn SetTexttoNull)