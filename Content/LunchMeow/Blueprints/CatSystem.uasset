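; CatSystem is a two-seat rocket pod that loads cat AI and launches them upward.
; Each detect box overlapping a BP_AI hides that actor, reveals a seated stand-in cat, waits briefly, then plays a timeline.
; The timeline adds a lerped upward offset to the chair every update, so movement accumulates, and sets that seat's finished flag.
; BeginPlay caches the tagged Cat1 and Cat2 actors, which are otherwise unused here.
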(event OnComponentBeginOverlap(DetectBox)
  (params (OverlappedComponent :type Primitive%20Component%20Object%20Reference) (OtherActor :type Actor%20Object%20Reference) (OtherComp :type Primitive%20Component%20Object%20Reference) (OtherBodyIndex :type Integer) (bFromSweep :type Boolean) (SweepResult :type Hit%20Result%20Structure%20%28by%20ref%29))
  ;[0.15 0.15 0.15 0.5] 火箭仓1
  (bind _asbp_ai (Utilities|Casting|CastToBP_AI OtherActor))
  ;;[0.15 0.15 0.15 0.5] 隐藏抓着的猫显示座椅猫
  (Rendering|SetActorHiddenInGame _asbp_ai true)
  (Rendering|SetVisibility (Variables|Default|GetCatReplace) true false)
  ;;[0.15 0.15 0.15 0.5] 等待一段时间发射猫咪
  (Utilities|FlowControl|Delay 1.5)
  (bind _moveup (Timeline|MoveUPTimeline PlayFromStart)
    (:Update
      (Transformation|AddLocalOffset (Variables|Default|GetChair1) (Math|Vector|Lerp(Vector) "0, 0, 0" "0.000000,0.000000,300.000000" _moveup) false false)
      (Variables|Default|SetIsSeat1Finish true))))

(event OnComponentEndOverlap(DetectBox)
  (params (OverlappedComponent :type Primitive%20Component%20Object%20Reference) (OtherActor :type Actor%20Object%20Reference) (OtherComp :type Primitive%20Component%20Object%20Reference) (OtherBodyIndex :type Integer))
  ;[0.15 0.15 0.15 0.5] 火箭仓1
)

(event OnComponentBeginOverlap(DetectBox2)
  (params (OverlappedComponent :type Primitive%20Component%20Object%20Reference) (OtherActor :type Actor%20Object%20Reference) (OtherComp :type Primitive%20Component%20Object%20Reference) (OtherBodyIndex :type Integer) (bFromSweep :type Boolean) (SweepResult :type Hit%20Result%20Structure%20%28by%20ref%29))
  ;[0.15 0.15 0.15 0.5] 火箭仓2
  (bind _asbp_ai (Utilities|Casting|CastToBP_AI OtherActor))
  ;;[0.15 0.15 0.15 0.5] 隐藏抓着的猫显示座椅猫
  (Rendering|SetActorHiddenInGame _asbp_ai true)
  (Rendering|SetVisibility (Variables|Default|GetCatReplace2) true false)
  ;;[0.15 0.15 0.15 0.5] 等待一段时间发射猫咪
  (Utilities|FlowControl|Delay 1.5)
  (bind _moveup (Timeline|MoveUPTimeline2 PlayFromStart)
    (:Update
      (Transformation|AddLocalOffset (Variables|Default|GetChair2) (Math|Vector|Lerp(Vector) "0, 0, 0" "0.000000,0.000000,300.000000" _moveup) false false)
      (Variables|Default|SetIsSeat2Finish true))))

(event OnComponentEndOverlap(DetectBox2)
  (params (OverlappedComponent :type Primitive%20Component%20Object%20Reference) (OtherActor :type Actor%20Object%20Reference) (OtherComp :type Primitive%20Component%20Object%20Reference) (OtherBodyIndex :type Integer))
  ;[0.15 0.15 0.15 0.5] 火箭仓2
)

(event EventBeginPlay
  (bind _outactors (Actor|GetAllActorswithTag "Cat1"))
  (Variables|Default|SetCat1 (Utilities|Array|Get(acopy) _outactors))
  (bind _outactors_2 (Actor|GetAllActorswithTag "Cat2"))
  (Variables|Default|SetCat2 (Utilities|Array|Get(acopy) _outactors_2)))

(event Collision|EventActorBeginOverlap
  (params (OtherActor :type Actor%20Object%20Reference)))

(event EventTick
  (params (DeltaSeconds :type Float%20%28single-precision%29)))

(fn ConstructionScript)