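; WholeRoket is the assembled rocket actor, built from Head, Body and Tail mesh components.
; UpdateWholeRokcet copies the mesh and first material of each part from the RoketDesk reference RD.
; The logic that sets RD, switches off the player camera and moves the parts by timeline is disconnected, as is the explosion activation.
; BeginPlay and the IsLunch check on Tick do nothing.
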(event Custom|UpdateWholeRokcet
  (bind _rd (Variables|Default|GetRD))
  (bind _rd_2 (Variables|Default|GetRD))
  (bind _head (Variables|Default|GetHead))
  (bind _rd_3 (Variables|Default|GetRD))
  (bind _body (Variables|Default|GetBody))
  (bind _tail (Variables|Default|GetTail))
  (bind _head_2 (Variables|/Game/LunchMeow/Blueprints/RoketDesk.RoketDesk_C|GetHead _rd_2))
  (bind _body_2 (Variables|/Game/LunchMeow/Blueprints/RoketDesk.RoketDesk_C|GetBody _rd_3))
  (bind _bottom (Variables|/Game/LunchMeow/Blueprints/RoketDesk.RoketDesk_C|GetBottom _rd))
  ;[0.15 0.15 0.15 0.5] 更新头部
  (Components|StaticMesh|SetStaticMesh _head (Variables|/Script/Engine.StaticMeshComponent|GetStaticMesh _head_2))
  (Rendering|Material|SetMaterial _head 0 (Rendering|Material|GetMaterial _head_2 0))
  ;[0.15 0.15 0.15 0.5] 更新身体
  (Components|StaticMesh|SetStaticMesh _body (Variables|/Script/Engine.StaticMeshComponent|GetStaticMesh _body_2))
  (Rendering|Material|SetMaterial _body 0 (Rendering|Material|GetMaterial _body_2 0))
  ;[0.15 0.15 0.15 0.5] 更新尾部
  (Components|StaticMesh|SetStaticMesh _tail (Variables|/Script/Engine.StaticMeshComponent|GetStaticMesh _bottom))
  (Rendering|Material|SetMaterial _tail 0 (Rendering|Material|GetMaterial _bottom 0)))

(event EventBeginPlay)

(event EventTick
  (params (DeltaSeconds :type Float%20%28single-precision%29))
  (Utilities|FlowControl|Sequence
    (:then_0
      (if (Variables|Default|GetIsLunch)
        _))))

(fn ConstructionScript)