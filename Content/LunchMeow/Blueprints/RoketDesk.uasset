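; Rocket-building desk where the player assembles a rocket from swappable head, body and bottom parts.
; Buttons cycle section and part indices; Tick shows that section's options and swaps the rocket's mesh and material.
; Confirm works after two Left clicks, then a timeline lerps the spring arm to top-down, restores movement and UI, and updates WholeRoket.
; A box overlap sets CanBuild; the first-person entry logic here is disconnected.
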(event OnClicked(Left)
  (params (TouchedComponent :type Primitive%20Component%20Object%20Reference) (ButtonPressed :type Key%20Structure :default "None"))
  ;[0.15 0.15 0.15 0.5] 选择火箭按钮
  (Variables|Default|SetRockClick (+ (Variables|Default|GetRockClick) 1))
  (if (<= (Variables|Default|GetSelectedRocketIndex) 2)
    (bind _output_get (Variables|Default|SetSelectedRocketIndex (+ (Variables|Default|GetSelectedRocketIndex) 1)))
    (Development|PrintString (Utilities|String|ToString(Integer) _output_get))
    (else
      (Variables|Default|SetSelectedRocketIndex 0))))

(event OnClicked(Down)
  (params (TouchedComponent :type Primitive%20Component%20Object%20Reference) (ButtonPressed :type Key%20Structure :default "None"))
  ;[0.15 0.15 0.15 0.5] 选择零件按钮
  (if (<= (Variables|Default|GetSelectedReplaceIndex) (Variables|Default|GetMaxSelectedReplaceIndex))
    (bind _output_get (Variables|Default|SetSelectedReplaceIndex (+ (Variables|Default|GetSelectedReplaceIndex) 1)))
    (Development|PrintString (Utilities|String|ToString(Integer) _output_get))
    (else
      (Variables|Default|SetSelectedReplaceIndex 0))))

(event OnComponentEndOverlap(Box)
  (params (OverlappedComponent :type Primitive%20Component%20Object%20Reference) (OtherActor :type Actor%20Object%20Reference) (OtherComp :type Primitive%20Component%20Object%20Reference) (OtherBodyIndex :type Integer))
  ;[0.15 0.15 0.15 0.5] 进出盒子开关提示
  (Utilities|Casting|CastToBP_TopDownCharacter OtherActor)
  (Variables|Default|SetCanBuild false))

(event OnClicked(Right)
  (params (TouchedComponent :type Primitive%20Component%20Object%20Reference) (ButtonPressed :type Key%20Structure :default "None"))
  ;[0.15 0.15 0.15 0.5] 选择火箭按钮
  (if (>= (Variables|Default|GetSelectedRocketIndex) 0)
    (Variables|Default|SetSelectedRocketIndex (- (Variables|Default|GetSelectedRocketIndex) 1))
    (else
      (Variables|Default|SetSelectedRocketIndex 2))))

(event OnComponentBeginOverlap(Box)
  (params (OverlappedComponent :type Primitive%20Component%20Object%20Reference) (OtherActor :type Actor%20Object%20Reference) (OtherComp :type Primitive%20Component%20Object%20Reference) (OtherBodyIndex :type Integer) (bFromSweep :type Boolean) (SweepResult :type Hit%20Result%20Structure%20%28by%20ref%29))
  ;[0.15 0.15 0.15 0.5] 进出盒子开关提示
  (bind _asbp_top_down_character (Utilities|Casting|CastToBP_TopDownCharacter OtherActor))
  (Development|PrintString (Utilities|GetDisplayName _asbp_top_down_character))
  (Variables|Default|SetCanBuild true))

(event OnClicked(Up)
  (params (TouchedComponent :type Primitive%20Component%20Object%20Reference) (ButtonPressed :type Key%20Structure :default "None"))
  ;[0.15 0.15 0.15 0.5] 选择零件按钮
  (if (>= (Variables|Default|GetSelectedReplaceIndex) 0)
    (Variables|Default|SetSelectedReplaceIndex (- (Variables|Default|GetSelectedReplaceIndex) 1))
    (else
      (Variables|Default|SetSelectedReplaceIndex (Variables|Default|GetMaxSelectedReplaceIndex)))))

(event OnClicked(Comfirm)
  (params (TouchedComponent :type Primitive%20Component%20Object%20Reference) (ButtonPressed :type Key%20Structure :default "None"))
  ;[0.15 0.15 0.15 0.5] 火箭完成按钮
  (if (Variables|Default|GetIfRocketFinish)
    (Development|PrintString "火箭制造成功")
    ;;[0.15 0.15 0.15 0.5] 改变视角到topdown
    (bind _camerazoomin (Timeline|Timeline_1 PlayFromStart)
      (:Update
        (CallFunction|ChangeViewtoTopDown _camerazoomin)
        (Variables|Default|SetStartBuilding false)
        (Default|ShowUI (Variables|Default|GetPlayerController))
        (Variables|/Game/TopDown/Blueprints/BP_TopDownController.BP_TopDownController_C|SetIsMovable (Variables|Default|GetPlayerController) true)
        (Variables|Default|SetFInishBuild true)
        (Default|UpdateWholeRokcet (Variables|Default|GetWholeRoket))))
    (else
      (Development|PrintString "火箭制造未完成"))))

(event EventBeginPlay
  (Utilities|FlowControl|Sequence
    (:then_0
      ;[0.15 0.15 0.15 0.5] 获得玩家
      (bind _returnvalue (Actor|GetActorOfClass "/Game/TopDown/Blueprints/BP_TopDownCharacter.BP_TopDownCharacter_C"))
      (Variables|Default|SetPlayerCharacter _returnvalue)
      (bind _returnvalue_2 (Actor|GetActorOfClass "/Game/TopDown/Blueprints/BP_TopDownController.BP_TopDownController_C"))
      (Variables|Default|SetPlayerController _returnvalue_2)
      (bind _returnvalue_3 (Actor|GetActorOfClass "/Game/LunchMeow/Blueprints/WholeRoket.WholeRoket_C"))
      (Variables|Default|SetWholeRoket _returnvalue_3))
    (:then_1
      ;[0.15 0.15 0.15 0.5] 获取火箭制作桌
      (bind _outactors (Actor|GetAllActorswithTag "RoketDesk"))
      (Variables|Default|SetRocketBuildDesk (Utilities|Array|Get(acopy) _outactors)))
    (:then_2
      ;[0.15 0.15 0.15 0.5] 隐藏所有可替换零件
      (CallFunction|HideReplace)
      (CallFunction|HideReplace 1)
      (CallFunction|HideReplace 2))))

(event EventTick
  (params (DeltaSeconds :type Float%20%28single-precision%29))
  (bind _selectedreplaceindex (Variables|Default|GetSelectedReplaceIndex))
  (bind _selectedreplaceindex_2 (Variables|Default|GetSelectedReplaceIndex))
  (bind _selectedreplaceindex_3 (Variables|Default|GetSelectedReplaceIndex))
  (bind _selectedrocketindex (Variables|Default|GetSelectedRocketIndex))
  (Utilities|FlowControl|Sequence
    (:then_0
      ;[0.15 0.15 0.15 0.5] 选择火箭逻辑
      (CallFunction|UpdateRocket _selectedrocketindex)
      (CallFunction|UpdateReplaceLine _selectedrocketindex))
    (:then_1
      ;[0.15 0.15 0.15 0.5] 选择零件替换逻辑(Head)
      (if (== (Variables|Default|GetSelectedRocketIndex) 0)
        ;;[0.15 0.15 0.15 0.5] 最大步数2
        (Variables|Default|SetMaxSelectedReplaceIndex 0)
        (CallFunction|UpdateReplace(Head) _selectedreplaceindex "/Game/A_LaunchMeow/Art/VFX/M_HighLight_Inst.M_HighLight_Inst" "/Engine/MapTemplates/Materials/BasicAsset01.BasicAsset01")
        (CallFunction|ReplaceRockettoParts(Head) _selectedreplaceindex)))
    (:then_2
      ;[0.15 0.15 0.15 0.5] 选择零件替换逻辑(Body)
      (if (== (Variables|Default|GetSelectedRocketIndex) 1)
        ;;[0.15 0.15 0.15 0.5] 最大步数3
        (Variables|Default|SetMaxSelectedReplaceIndex 1)
        (CallFunction|UpdateReplace(Body) _selectedreplaceindex_2 "/Game/A_LaunchMeow/Art/VFX/M_HighLight_Inst.M_HighLight_Inst" 0 "/Engine/MapTemplates/Materials/BasicAsset01.BasicAsset01")
        (CallFunction|ReplaceRockettoParts(Body) _selectedreplaceindex_2)))
    (:then_3
      ;[0.15 0.15 0.15 0.5] 选择零件替换逻辑(Bottom)
      (if (== (Variables|Default|GetSelectedRocketIndex) 2)
        ;;[0.15 0.15 0.15 0.5] 最大步数2
        (Variables|Default|SetMaxSelectedReplaceIndex 0)
        (CallFunction|UpdateReplace(Bottom) _selectedreplaceindex_3 "/Game/A_LaunchMeow/Art/VFX/M_HighLight_Inst.M_HighLight_Inst")
        (CallFunction|ReplaceRockettoParts(Bottom) _selectedreplaceindex_3)))
    (:then_4
      ;[0.15 0.15 0.15 0.5] 判断火箭制作是否完成
      (if (>= (Variables|Default|GetRockClick) 2)
        (Variables|Default|SetIfRocketFinish true)))))

(fn ConstructionScript)

(fn UpdateRocket
  (params (SelectIndex :type Integer))
  (Utilities|FlowControl|Sequence
    (:then_0
      (if (== SelectIndex 0)
        (Rendering|Material|SetMaterial (Variables|Default|GetHead) 0 "/Engine/MapTemplates/Materials/BasicAsset01.BasicAsset01")))
    (:then_1
      (if (== SelectIndex 1)
        (Rendering|Material|SetMaterial (Variables|Default|GetBody) 0 "/Engine/MapTemplates/Materials/BasicAsset01.BasicAsset01")))
    (:then_2
      (if (== SelectIndex 2)
        (Rendering|Material|SetMaterial (Variables|Default|GetBottom) 0 "/Engine/MapTemplates/Materials/BasicAsset01.BasicAsset01")))))

(fn UpdateReplace(Head)
  (params (SelectIndex :type Integer) (OverlayMaterial :type Material%20Instance%20Object%20Reference) (HightLightMaterial :type Material%20Object%20Reference))
  (bind _headpart0 (Variables|Default|GetHeadPart0))
  (bind _headpart1 (Variables|Default|GetHeadPart1))
  (Utilities|FlowControl|Sequence
    (:then_0
      (if (== SelectIndex 0)
        (Rendering|Material|SetOverlayMaterial _headpart0 OverlayMaterial :!class /Script/Engine.MeshComponent)
        (Rendering|Material|SetOverlayMaterialMaxDrawDistance _headpart0 1e+27 :!class /Script/Engine.MeshComponent)))
    (:then_1
      (if (== SelectIndex 1)
        (Rendering|Material|SetOverlayMaterial _headpart1 OverlayMaterial :!class /Script/Engine.MeshComponent)
        (Rendering|Material|SetOverlayMaterialMaxDrawDistance _headpart1 1e+27 :!class /Script/Engine.MeshComponent)))))

(fn HideReplace
  (params (Index :type Integer))
  (bind _bottompart1 (Variables|Default|GetBottomPart1))
  (bind _headpart0 (Variables|Default|GetHeadPart0))
  (bind _bodypart0 (Variables|Default|GetBodyPart0))
  (Utilities|FlowControl|Sequence
    (:then_0
      (if (== Index 0)
        (Rendering|SetVisibility _headpart0 false false)
        (Collision|SetCollisionEnabled _headpart0 "NoCollision")))
    (:then_1
      (if (== Index 1)
        (Rendering|SetVisibility _bodypart0 false false)
        (Collision|SetCollisionEnabled _bodypart0 "NoCollision")))
    (:then_2
      (if (== Index 2)
        (Rendering|SetVisibility _bottompart1 false false)
        (Collision|SetCollisionEnabled _bottompart1 "NoCollision")))))

(fn ShowReplace
  (params (Index :type Integer))
  (bind _bottompart1 (Variables|Default|GetBottomPart1))
  (bind _headpart0 (Variables|Default|GetHeadPart0))
  (bind _bodypart0 (Variables|Default|GetBodyPart0))
  (Utilities|FlowControl|Sequence
    (:then_0
      (if (== Index 0)
        (Rendering|SetVisibility _headpart0 true false)
        (Collision|SetCollisionEnabled _headpart0 "NoCollision")))
    (:then_1
      (if (== Index 1)
        (Rendering|SetVisibility _bodypart0 true false)
        (Collision|SetCollisionEnabled _bodypart0 "NoCollision")))
    (:then_2
      (if (== Index 2)
        (Rendering|SetVisibility _bottompart1 true false)
        (Collision|SetCollisionEnabled _bottompart1 "NoCollision")))))

(fn UpdateReplaceLine
  (params (SelectIndex :type Integer))
  (Utilities|FlowControl|Sequence
    (:then_0
      (if (== SelectIndex 0)
        (CallFunction|ShowReplace)
        (CallFunction|HideReplace 1)
        (CallFunction|HideReplace 2)))
    (:then_1
      (if (== SelectIndex 1)
        (CallFunction|ShowReplace 1)
        (CallFunction|HideReplace)
        (CallFunction|HideReplace 2)))
    (:then_2
      (if (== SelectIndex 2)
        (CallFunction|ShowReplace 2)
        (CallFunction|HideReplace 1)
        (CallFunction|HideReplace)))))

(fn ReplaceRockettoParts(Head)
  (params (SelectIndex :type Integer))
  (bind _head (Variables|Default|GetHead))
  (bind _head_2 (Variables|Default|GetHead))
  (Utilities|FlowControl|Sequence
    (:then_0
      (if (== SelectIndex 0)
        (Components|StaticMesh|SetStaticMesh _head "/Game/LunchMeow/Mushes/Rokcet/SM_WoodHead.SM_WoodHead")
        (Rendering|Material|SetMaterial _head 0 "/Game/LunchMeow/Mushes/Rokcet/MAT_WoodHead.MAT_WoodHead")))
    (:then_1
      (if (== SelectIndex 1)
        (Components|StaticMesh|SetStaticMesh _head_2 "/Game/LunchMeow/Mushes/Rokcet/GreenHead.GreenHead")
        (Rendering|Material|SetMaterial _head_2 0 "/Game/LunchMeow/Mushes/Rokcet/MAT_YellowHead.MAT_YellowHead")))))

(fn ReplaceRockettoParts(Body)
  (params (SelectIndex :type Integer))
  (bind _body (Variables|Default|GetBody))
  (bind _body_2 (Variables|Default|GetBody))
  (bind _body_3 (Variables|Default|GetBody))
  (Utilities|FlowControl|Sequence
    (:then_0
      (if (== SelectIndex 0)
        (Components|StaticMesh|SetStaticMesh _body_2 "/Game/LunchMeow/Mushes/Rokcet/SM_WoodBody.SM_WoodBody")
        (Rendering|Material|SetMaterial _body_2 0 "/Game/LunchMeow/Mushes/Rokcet/MAT_WoodBody.MAT_WoodBody")))
    (:then_1
      (if (== SelectIndex 1)
        (Components|StaticMesh|SetStaticMesh _body_3 "/Game/LunchMeow/Mushes/Rokcet/YellowBody.YellowBody")
        (Rendering|Material|SetMaterial _body_3 0 "/Game/LunchMeow/Mushes/Rokcet/MAT_YellowBody.MAT_YellowBody")))
    (:then_2
      (if (== SelectIndex 2)
        (Components|StaticMesh|SetStaticMesh _body "/Game/LunchMeow/Mushes/Rokcet/SM_ArtBody.SM_ArtBody")
        (Rendering|Material|SetMaterial _body 0 "/Game/LunchMeow/Mushes/Rokcet/MAT_ArtBody.MAT_ArtBody")))))

(fn ReplaceRockettoParts(Bottom)
  (params (SelectIndex :type Integer))
  (bind _bottom (Variables|Default|GetBottom))
  (bind _bottom_2 (Variables|Default|GetBottom))
  (Utilities|FlowControl|Sequence
    (:then_0
      (if (== SelectIndex 0)
        (Components|StaticMesh|SetStaticMesh _bottom_2 "/Game/LunchMeow/Mushes/Rokcet/SM_WoodTail.SM_WoodTail")
        (Rendering|Material|SetMaterial _bottom_2 0 "/Game/LunchMeow/Mushes/Rokcet/MAT_WoodTial.MAT_WoodTial")))
    (:then_1
      (if (== SelectIndex 1)
        (Components|StaticMesh|SetStaticMesh _bottom "/Game/LunchMeow/Mushes/Rokcet/YellowTail.YellowTail")
        (Rendering|Material|SetMaterial _bottom 0 "/Game/LunchMeow/Mushes/Rokcet/MAT_YellowTail.MAT_YellowTail")))))

(fn UpdateReplace(Body)
  (params (SelectIndex :type Integer) (OverlayMaterial :type Material%20Instance%20Object%20Reference) (DefaultMaterial :type Material%20Object%20Reference) (HIghlightMaterial :type Material%20Object%20Reference))
  (bind _bodypart2 (Variables|Default|GetBodyPart2))
  (bind _bodypart0 (Variables|Default|GetBodyPart0))
  (Utilities|FlowControl|Sequence
    (:then_0
      (if (== SelectIndex 0)
        (Rendering|Material|SetOverlayMaterial _bodypart0 0 :!class /Script/Engine.MeshComponent)
        (Rendering|Material|SetOverlayMaterialMaxDrawDistance _bodypart0 1e+27 :!class /Script/Engine.MeshComponent)))
    (:then_1
      (if (== SelectIndex 1)
        (Rendering|Material|SetOverlayMaterial (Variables|Default|GetBodyPart1) 0 :!class /Script/Engine.MeshComponent)))
    (:then_2
      (if (== SelectIndex 2)
        (Rendering|Material|SetOverlayMaterial _bodypart2 0 :!class /Script/Engine.MeshComponent)
        (Rendering|Material|SetOverlayMaterialMaxDrawDistance _bodypart2 1e+27 :!class /Script/Engine.MeshComponent)))))

(fn UpdateReplace(Bottom)
  (params (SelectIndex :type Integer) (OverlayMaterial :type Material%20Instance%20Object%20Reference) (HeighlightMaterial :type Material%20Object%20Reference) (DefaultMaterial :type Material%20Object%20Reference))
  (bind _bottompart1 (Variables|Default|GetBottomPart1))
  (bind _bottompart0 (Variables|Default|GetBottomPart0))
  (Utilities|FlowControl|Sequence
    (:then_0
      (if (== SelectIndex 0)
        (Rendering|Material|SetOverlayMaterial _bottompart0 0 :!class /Script/Engine.MeshComponent)
        (Rendering|Material|SetOverlayMaterialMaxDrawDistance _bottompart0 1e+27 :!class /Script/Engine.MeshComponent)))
    (:then_1
      (if (== SelectIndex 1)
        (Rendering|Material|SetOverlayMaterial _bottompart1 0 :!class /Script/Engine.MeshComponent)
        (Rendering|Material|SetOverlayMaterialMaxDrawDistance _bottompart1 1e+27 :!class /Script/Engine.MeshComponent)))))

(fn ChangeViewtoFirstPerson
  (params (Alpha :type Float%20%28double-precision%29))
  (bind _playercharacter (Variables|Default|GetPlayerCharacter))
  (bind _springarm (Variables|/Game/TopDown/Blueprints/BP_TopDownCharacter.BP_TopDownCharacter_C|GetSpringArm _playercharacter))
  (Utilities|FlowControl|Sequence
    (:then_0
      ;[0.15 0.15 0.15 0.5] 调整远近
      (Variables|/Script/Engine.SpringArmComponent|SetTargetArmLength _springarm (Math|Float|Lerp (Variables|Default|GetTopDownLength) (Variables|Default|GetFirstPersonLength) Alpha)))
    (:then_1
      ;[0.15 0.15 0.15 0.5] 微调距离
      (Variables|/Script/Engine.SpringArmComponent|SetSocketOffset _springarm (Math|Vector|Lerp(Vector) (Variables|Default|GetTopDownOffset) (Variables|Default|GetFirstPersonOffset) Alpha)))
    (:then_2
      ;[0.15 0.15 0.15 0.5] 调整垂直角度
      (Transformation|SetWorldRotation _springarm (Math|Rotator|Lerp(Rotator) (Math|Rotator|MakeRotator 0.0 -5e+01 0.0) (Math|Rotator|MakeRotator 0.0 0.0 0.0) Alpha) false false))))

(fn ChangeViewtoTopDown
  (params (Alpha :type Float%20%28double-precision%29))
  (bind _playercharacter (Variables|Default|GetPlayerCharacter))
  (bind _springarm (Variables|/Game/TopDown/Blueprints/BP_TopDownCharacter.BP_TopDownCharacter_C|GetSpringArm _playercharacter))
  (Utilities|FlowControl|Sequence
    (:then_0
      ;[0.15 0.15 0.15 0.5] 调整远近
      (Variables|/Script/Engine.SpringArmComponent|SetTargetArmLength _springarm (Math|Float|Lerp (Variables|Default|GetFirstPersonLength) (Variables|Default|GetTopDownLength) Alpha)))
    (:then_1
      ;[0.15 0.15 0.15 0.5] 微调距离
      (Variables|/Script/Engine.SpringArmComponent|SetSocketOffset _springarm (Math|Vector|Lerp(Vector) (Variables|Default|GetFirstPersonOffset) (Variables|Default|GetTopDownOffset) Alpha)))
    (:then_2
      ;[0.15 0.15 0.15 0.5] 调整垂直角度
      (Transformation|SetWorldRotation _springarm (Math|Rotator|Lerp(Rotator) (Math|Rotator|MakeRotator 0.0 0.0 0.0) (Math|Rotator|MakeRotator 0.0 -5e+01 0.0) Alpha) false false))))