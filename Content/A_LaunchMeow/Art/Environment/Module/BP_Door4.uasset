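; BP_Door4 is a two-panel sliding door that triggers when a Character enters its Box and reverses automatically.
; Paired timelines move DoorTop and DoorDown along relative Z, then a second pair runs after a three-second delay, presumably closing it.
; Two DoOnce gates re-arm each other, so overlaps are ignored until the top panel finishes its return.
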(event OnComponentBeginOverlap(Box)
  (params (OverlappedComponent :type Primitive%20Component%20Object%20Reference) (OtherActor :type Actor%20Object%20Reference) (OtherComp :type Primitive%20Component%20Object%20Reference) (OtherBodyIndex :type Integer) (bFromSweep :type Boolean) (SweepResult :type Hit%20Result%20Structure%20%28by%20ref%29))
  (Utilities|Casting|CastToCharacter OtherActor)
  (Utilities|FlowControl|DoOnce false
    (:Completed
      (CallFunction|RestartClose)
      (Utilities|FlowControl|Sequence
        (:then_0
          (bind _newtrack_0 (Timeline|Timeline PlayFromStart)
            (:Update
              (Transformation|SetRelativeLocation (Variables|Default|GetDoor_Top) (Math|Vector|MakeVector 0.0 0.0 _newtrack_0) false false))
            (:Finished
              (Utilities|FlowControl|Delay 3.0)
              (Utilities|FlowControl|DoOnce false
                (:Completed
                  (Utilities|FlowControl|Sequence
                    (:then_0
                      (bind _newtrack_0_2 (Timeline|Timeline_1 PlayFromStart)
                        (:Update
                          (Transformation|SetRelativeLocation (Variables|Default|GetDoor_Top) (Math|Vector|MakeVector 0.0 0.0 _newtrack_0_2) false false))
                        (:Finished
                          (CallFunction|RestartOpen))))
                    (:then_1
                      (bind _newtrack_0_3 (Timeline|Timeline_2 PlayFromStart)
                        (:Update
                          (Transformation|SetRelativeLocation (Variables|Default|GetDoor_Down) (Math|Vector|MakeVector 0.0 0.0 _newtrack_0_3) false false))))))))))
        (:then_1
          (bind _newtrack_0_4 (Timeline|Timeline_0 PlayFromStart)
            (:Update
              (Transformation|SetRelativeLocation (Variables|Default|GetDoor_Down) (Math|Vector|MakeVector 0.0 0.0 _newtrack_0_4) false false))))))))

(event Custom|RestartClose
  (Utilities|FlowControl|DoOnce false) ; enters at Reset
)

(event Custom|RestartOpen
  (Utilities|FlowControl|DoOnce false) ; enters at Reset
)

(event EventBeginPlay
  (Utilities|FlowControl|Delay 1.0))

(event Collision|EventActorBeginOverlap
  (params (OtherActor :type Actor%20Object%20Reference)))

(event EventTick
  (params (DeltaSeconds :type Float%20%28single-precision%29)))

(fn ConstructionScript)