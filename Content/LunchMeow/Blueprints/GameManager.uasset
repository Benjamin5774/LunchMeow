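; GameManager steps the LunchMeow player through the launch preparation flow, from talking to Alice to rocket assembly, cat selection and launch.
; BeginPlay caches the UI, desk, dialogue, cat, character and controller actors via GetActorOfClass.
; Tick enables the Alice conversation, then polls dialogue, rocket build and both cat seat states.
; Each milestone passes a DoOnce gate and briefly raises its guidance flag using timed delays.
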(event EventBeginPlay
  ;[0.15 0.15 0.15 0.5] 初始化一切
  (bind _returnvalue (Actor|GetActorOfClass "/Game/LunchMeow/Blueprints/UISystem.UISystem_C"))
  (Variables|Default|SetUISystem _returnvalue)
  (bind _returnvalue_2 (Actor|GetActorOfClass "/Game/LunchMeow/Blueprints/LunchDesk.LunchDesk_C"))
  (Variables|Default|SetLunchDesk _returnvalue_2)
  (bind _returnvalue_3 (Actor|GetActorOfClass "/Game/LunchMeow/Blueprints/RoketDesk.RoketDesk_C"))
  (Variables|Default|SetRoketDesk _returnvalue_3)
  (bind _returnvalue_4 (Actor|GetActorOfClass "/Game/TopDown/Blueprints/BP_TopDownCharacter.BP_TopDownCharacter_C"))
  (Variables|Default|SetPlayerCharacter _returnvalue_4)
  (bind _returnvalue_5 (Actor|GetActorOfClass "/Game/LunchMeow/Blueprints/DialogueSystem.DialogueSystem_C"))
  (Variables|Default|SetDialogueSystem _returnvalue_5)
  (bind _returnvalue_6 (Actor|GetActorOfClass "/Game/TopDown/Blueprints/BP_TopDownController.BP_TopDownController_C"))
  (Variables|Default|SetPlayerController _returnvalue_6)
  (bind _returnvalue_7 (Actor|GetActorOfClass "/Game/LunchMeow/Blueprints/CatSystem.CatSystem_C"))
  (Variables|Default|SetCatSystem _returnvalue_7))

(event EventTick
  (params (DeltaSeconds :type Float%20%28single-precision%29))
  (bind _catsystem (Variables|Default|GetCatSystem))
  (Utilities|FlowControl|Sequence
    (:then_0
      ;[0.15 0.15 0.15 0.5] Alice对话
      (Utilities|FlowControl|DoOnce false
        (:Completed
          (Variables|Default|SetCanTalk true)
          (Variables|/Game/LunchMeow/Blueprints/DialogueSystem.DialogueSystem_C|SetIsTalkToAlice (Variables|Default|GetDialogueSystem) true))))
    (:then_1
      ;[0.15 0.15 0.15 0.5] 指引去火箭组装
      (if (not (Variables|/Game/LunchMeow/Blueprints/DialogueSystem.DialogueSystem_C|GetIsTalkToAlice (Variables|Default|GetDialogueSystem)))
        (Utilities|FlowControl|DoOnce false
          (:Completed
            (Variables|Default|SetGuidanceToRocketDesk true)
            (Utilities|FlowControl|Delay 3.0)
            (Variables|Default|SetGuidanceToRocketDesk false)))))
    (:then_2
      ;[0.15 0.15 0.15 0.5] 指引去选猫
      (if (Variables|/Game/LunchMeow/Blueprints/RoketDesk.RoketDesk_C|GetFInishBuild (Variables|Default|GetRoketDesk))
        (Utilities|FlowControl|DoOnce false
          (:Completed
            (Variables|Default|SetGuidanceToCatRoom true)
            (Utilities|FlowControl|Delay 3.0)
            (Variables|Default|SetGuidanceToCatRoom false)))))
    (:then_3
      ;[0.15 0.15 0.15 0.5] 指引去发射
      (if (and (Variables|/Game/LunchMeow/Blueprints/CatSystem.CatSystem_C|GetIsSeat1Finish _catsystem) (Variables|/Game/LunchMeow/Blueprints/CatSystem.CatSystem_C|GetIsSeat2Finish _catsystem))
        (Utilities|FlowControl|DoOnce false
          (:Completed
            (Utilities|FlowControl|Delay 1.0)
            (Variables|Default|SetGuidanceToLunchRoom true)
            (Utilities|FlowControl|Delay 3.0)
            (Variables|Default|SetGuidanceToLunchRoom false)))))))

(fn ConstructionScript)