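; BP_AI_INFP is a scripted AI pawn that walks a fixed route and ends in an arguing pose.
; BeginPlay chains two AIMoveTo calls to hard-coded points, then rotates the mesh and loops the Standing_Arguing animation.
; While the NewVar flag is true, Tick forces a fixed world rotation on the mesh; reaching the first point clears the flag.
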(event EventBeginPlay
  (bind _self self)
  (AI|AIMoveTo _self "-2835.000000,-495.411733,1203.222485" 0 2.0 false
    (:OnSuccess
      (Variables|Default|SetNewVar false)
      (AI|AIMoveTo _self "-2530.000000,-175.000000,1203.222485" 0 5.0 false
        (:OnSuccess
          (Transformation|SetWorldRotation (Variables|Character|GetMesh) "0.000000,90.000000,0.000000" false false)
          (Components|Animation|PlayAnimation (Variables|Character|GetMesh) "/Game/A_LaunchMeow/Art/Animation/Cat/AI/Standing_Arguing.Standing_Arguing" true))))))

(event Collision|EventActorBeginOverlap
  (params (OtherActor :type Actor%20Object%20Reference)))

(event EventTick
  (params (DeltaSeconds :type Float%20%28single-precision%29))
  (if (Variables|Default|GetNewVar)
    (Transformation|SetWorldRotation (Variables|Character|GetMesh) "0.000000,-90.000000,0.000000" false false)))

(fn ConstructionScript)